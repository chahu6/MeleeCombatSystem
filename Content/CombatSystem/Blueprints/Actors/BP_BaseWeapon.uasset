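; BP_BaseWeapon is the base equippable weapon actor for the combat system, dealing damage to what it strikes.
; On equip it attaches to the hand or holster socket by combat state, registers as main weapon, and sends its combat type to the character's AnimInstance.
; Its collision component uses the item mesh, ignores the owner, and applies point damage to hit actors not reported dead.
; It can also switch the mesh to physics simulation.
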(event `self.AC_CollisionComponent.OnHit`
  (params (HitResult :type "HitResult Structure"))
  (set `self.HitActor` (`.HitActor` (`GameplayStatics.BreakHitResult` HitResult)))
  (bind _returnvalue (message `/Game/CombatSystem/Blueprints/Interfaces/BI_Combat.IsDead` (`self.HitActor`)))
  (if (not _returnvalue)
    (`GameplayStatics.ApplyPointDamage` (`self.HitActor`) (`self.Damage`) (`self.GetActorForwardVector` (`self.GetOwner`)) HitResult (`self.GetInstigatorController`) self)))

(event `SimulateWeaponPhysics`
  (bind _returnvalue (`self.GetItemMesh`))
  (`PrimitiveComponent.SetCollisionProfileName` _returnvalue "PhysicsActor" true)
  (`PrimitiveComponent.SetSimulatePhysics` _returnvalue true))

(fn `OnEquipped`
  (`parent.OnEquipped`)
  (set `self.CombatComponent` (`self.GetComponentByClass` (`self.GetOwner`) "/Game/CombatSystem/Blueprints/Components/AC_CombatComponent.AC_CombatComponent_C"))
  (`self.AttachToActor` (select `bool` (`/Game/CombatSystem/Blueprints/Components/AC_CombatComponent.IsCombatEnabled?` (`self.CombatComponent`)) :`false` (`self.Attach Socket Name`) :`true` (`self.HandSocketName`)))
  (`/Game/CombatSystem/Blueprints/Components/AC_CombatComponent.SetMainWeapon` (`self.CombatComponent`) self)
  (message `/Game/CombatSystem/Blueprints/Interfaces/BI_AnimInstance.UpdateCombatType` (`SkeletalMeshComponent.GetAnimInstance` (`Character.Mesh` (cast `/Game/CombatSystem/Blueprints/BP_CombatCharacter` (`self.GetOwner`) :!pure true))) (`self.CombatType`))
  (`/Game/CombatSystem/Blueprints/Components/AC_CollisionComponent.SetCollisionComponent` (`self.AC_CollisionComponent`) (`self.GetItemMesh`))
  (`/Game/CombatSystem/Blueprints/Components/AC_CollisionComponent.AddActorToIgnore` (`self.AC_CollisionComponent`) (`self.GetOwner`)))

(fn `UserConstructionScript`
  (`parent.UserConstructionScript`))