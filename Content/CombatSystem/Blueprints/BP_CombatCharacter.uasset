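; BP_CombatCharacter is a character that toggles a combat stance and interacts with nearby objects.
; The toggle input plays the main weapon's enter or exit montage and pushes the combat flag to the anim instance through an interface message.
; Interact runs a sphere trace at the character's location and messages the hit actor.
; Setting a new main weapon unequips and destroys the previous one before storing the replacement.
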(event `EnhancedInput|/Game/CombatSystem/Input/Actions/IA_ToggleCombat`
  (params (ActionValue :type Boolean) (ElapsedSeconds :type "Float (double-precision)") (TriggeredSeconds :type "Float (double-precision)") (InputAction :type "InputAction Object Reference" :default "/Game/CombatSystem/Input/Actions/IA_ToggleCombat.IA_ToggleCombat"))
  (:`Started`
    (if (not (`self.IsCombatEnabled?`))
      (`self.PlayAnimMontage` (`/Game/CombatSystem/Blueprints/Actors/BP_BaseWeapon.EnterCombat` (`self.MainWeapon`)))
      (`self.SetCombatEnabled` true)
      (else
        (`self.PlayAnimMontage` (`/Game/CombatSystem/Blueprints/Actors/BP_BaseWeapon.ExitCombat` (`self.MainWeapon`)))
        (`self.SetCombatEnabled` false)))))

(event `EnhancedInput|/Game/CombatSystem/Input/Actions/IA_Interact`
  (params (ActionValue :type Boolean) (ElapsedSeconds :type "Float (double-precision)") (TriggeredSeconds :type "Float (double-precision)") (InputAction :type "InputAction Object Reference" :default "/Game/CombatSystem/Input/Actions/IA_Interact.IA_Interact"))
  (bind _returnvalue (`self.K2_GetActorLocation`))
  (:`Started`
    (bind (_outhit _returnvalue_2) (`KismetSystemLibrary.SphereTraceSingleForObjects` :`Start` _returnvalue :`End` _returnvalue :`Radius` 100.0 :`ObjectTypes` (`|MakeArray` "ObjectTypeQuery7" :!type "EObjectTypeQuery Enum") :`DrawDebugType` "ForDuration"))
    (if _returnvalue_2
      (message `/Game/CombatSystem/Blueprints/Interfaces/BI_Interactable.Interact` (`.HitActor` (`GameplayStatics.BreakHitResult` _outhit)) self))))

(fn `GetMainWeapon`
  (returns (ReturnValue :type "/Game/CombatSystem/Blueprints/Actors/BP_BaseWeapon Object Reference"))
  (return (`self.MainWeapon`)))

(fn `IsCombatEnabled?`
  (returns (ReturnValue :type Boolean))
  (return (`self.bIsCombatEnabled?`)))

(fn `SetCombatEnabled`
  (params (`bIsCombatEnabled?` :type Boolean))
  (bind _output_get (set `self.bIsCombatEnabled?` `bIsCombatEnabled?`))
  (message `/Game/CombatSystem/Blueprints/Interfaces/BI_AnimInstance.UpdateCombatEnabled` (`SkeletalMeshComponent.GetAnimInstance` (`self.Mesh`)) _output_get))

(fn `SetMainWeapon`
  (params (NewWeapon :type "/Game/CombatSystem/Blueprints/Actors/BP_BaseWeapon Object Reference"))
  (`|ExecutionSequence`
    (:`then_0`
      (bind _mainweapon (`self.MainWeapon`)
        (:`then`
          (`/Game/CombatSystem/Blueprints/Actors/BP_BaseEquippable.OnUnEquipped` _mainweapon)
          (`self.K2_DestroyActor` _mainweapon))
        (:`else`)))
    (:`then_1`
      (set `self.MainWeapon` (`local.NewWeapon`)))))

(fn `UserConstructionScript`)