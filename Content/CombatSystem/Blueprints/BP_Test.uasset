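; BP_Test is a combat system test actor that spawns and equips its starting equipment when play begins.
; On BeginPlay it spawns each class in StartingEquipment at its own transform as owner and instigator, then calls OnEquipped on every valid spawned actor.
; Overlap and Tick events are disabled, and the construction script only calls its parent.
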(event `self.ReceiveBeginPlay`
  (`parent.ReceiveBeginPlay`)
  (for _array_element (`self.StartingEquipment`)
    (bind _returnvalue (`|SpawnActorFromClass` _array_element (`self.GetTransform`) "Undefined" "MultiplyWithRoot" self self))
    (`/Engine/EditorBlueprintResources/StandardMacros.IsValid` _returnvalue
      (:`Is Valid`
        (`/Game/CombatSystem/Blueprints/Actors/BP_BaseEquippable.OnEquipped` _returnvalue)))))

(fn `UserConstructionScript`
  (`parent.UserConstructionScript`))