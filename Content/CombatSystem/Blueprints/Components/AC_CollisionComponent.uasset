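; Actor component that performs hit detection for the combat system while its collision is enabled.
; Each tick it sphere-traces between two sockets on an assigned mesh, filtered by object types and an editable ignore list.
; Newly hit actors are recorded and reported through an OnHit call, so each is hit once per activation.
; Enabling collision clears that record, and getters expose the last hit and current state.
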(event `EnableCollision`
  (`self.ClearHitActors`)
  (set `self.bIsCollisionEnabled?` true))

(event `DisableCollision`
  (set `self.bIsCollisionEnabled?` false))

(event `ClearHitActors`
  (`KismetArrayLibrary.Array_Clear` (`self.AlreadyHitActors`)))

(event `self.ReceiveTick`
  (params (DeltaSeconds :type "Float (single-precision)"))
  (if (`self.bIsCollisionEnabled?`)
    (`self.CollisionTrace`)))

(event `CollisionTrace`
  (bind _collisionmeshcomponent (`self.CollisionMeshComponent`))
  (bind _outhits (`KismetSystemLibrary.SphereTraceMultiForObjects` (`SceneComponent.GetSocketLocation` _collisionmeshcomponent (`self.StartSocketName`)) (`SceneComponent.GetSocketLocation` _collisionmeshcomponent (`self.EndSocketName`)) (`self.TraceRadius`) (`self.CollisionObjectType`) false (`self.Actors to Ignore`) (`self.Draw Debug Type`)))
  (for _array_element _outhits
    (bind _output_get (set `self.LastHit` _array_element))
    (bind (_bblockinghit _binitialoverlap _time _distance _location _impactpoint _normal _impactnormal _physmat _hitactor) (`GameplayStatics.BreakHitResult` _output_get))
    (if (not (`KismetArrayLibrary.Array_Contains` (`self.AlreadyHitActors`) _hitactor))
      (bind _output_get_2 (set `self.HitActor` _hitactor))
      (`KismetArrayLibrary.Array_Add` (`self.AlreadyHitActors`) _output_get_2)
      (`self.OnHit` (`self.LastHit`)))))

(event `SetCollisionComponent`
  (params (CollisionMeshComponent :type "PrimitiveComponent Object Reference"))
  (set `self.CollisionMeshComponent` CollisionMeshComponent))

(fn `AddActorToIgnore`
  (params (InActor :type "Actor Object Reference (by ref)"))
  (`KismetArrayLibrary.Array_AddUnique` (`self.Actors to Ignore`) InActor))

(fn `GetActorsToIgnore`
  (returns (ReturenValue :type "Array of Actor Object Reference"))
  (return (`self.Actors to Ignore`)))

(fn `GetAlreadyHitActor`
  (returns (AlreadyHitActors :type "Array of Actor Object Reference"))
  (return (`self.AlreadyHitActors`)))

(fn `GetCollisionComponent`
  (returns (ReturnValue :type "PrimitiveComponent Object Reference"))
  (return (`self.CollisionMeshComponent`)))

(fn `GetLastHit`
  (returns (ReturnValue :type "HitResult Structure"))
  (return (`self.LastHit`)))

(fn `IsCollisionEnabled?`
  (returns (ReturnValue :type Boolean))
  (return (`self.bIsCollisionEnabled?`)))

(fn `RemoveActorToIgnore`
  (params (ActorToRemove :type "Actor Object Reference (by ref)"))
  (`KismetArrayLibrary.Array_RemoveItem` (`self.Actors to Ignore`) ActorToRemove))