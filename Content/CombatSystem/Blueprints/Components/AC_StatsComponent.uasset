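; Actor component for the combat system that stores a character's base, max and current stats and applies damage to Health.
; Current values initialize from the base map, and every write broadcasts OnCurrentStatValueUpdated; modifications clamp to max and can request regeneration.
; TakeDamage scales damage against Armor with a damage / (damage + armor) ratio.
; Only Stamina regenerates, through a looping timer that starts after a short delay and stops at max.
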(event `StartRegen`
  (params (StatType :type "/Game/CombatSystem/Blueprints/Enums/E_Stats Enum" :default "NewEnumerator0"))
  (switch `/Game/CombatSystem/Blueprints/Enums/E_Stats` StatType
    (:`NewEnumerator2`
      (`KismetSystemLibrary.K2_ClearTimer` null "RegenStamina")
      (`KismetSystemLibrary.Delay` 1.5)
      (`KismetSystemLibrary.K2_SetTimer` null "RegenStamina" 0.1 true))))

(fn `GetBaseStatValue`
  (params (Key :type "/Game/CombatSystem/Blueprints/Enums/E_Stats Enum" :default "NewEnumerator0"))
  (returns (ReturnValue :type "Float (double-precision)"))
  (return (break `/Game/CombatSystem/Blueprints/Structs/F_BaseStat` (`BlueprintMapLibrary.Map_Find` (`self.BaseStats`) Key))))

(fn `GetCurrentStatValue`
  (params (Key :type "/Game/CombatSystem/Blueprints/Enums/E_Stats Enum" :default "NewEnumerator0"))
  (returns (ReturnValue :type "Float (double-precision)"))
  (return (`BlueprintMapLibrary.Map_Find` (`self.CurrentStats`) Key)))

(fn `GetMaxStatValue`
  (params (Key :type "/Game/CombatSystem/Blueprints/Enums/E_Stats Enum" :default "NewEnumerator0"))
  (returns (ReturnValue :type "Float (double-precision)"))
  (return (`.MaxValue_5_873E80DC4EA29BDBBE9BD8B9FF68767F` (break `/Game/CombatSystem/Blueprints/Structs/F_BaseStat` (`BlueprintMapLibrary.Map_Find` (`self.BaseStats`) Key)))))

(fn `InitializeStatus`
  (bind _keys (`BlueprintMapLibrary.Map_Keys` (`self.BaseStats`)))
  (for _array_element _keys
    (`self.SetCurrentStatValue` _array_element (break `/Game/CombatSystem/Blueprints/Structs/F_BaseStat` (`BlueprintMapLibrary.Map_Find` (`self.BaseStats`) _array_element)))))

(fn `ModifyCurrentStatValue`
  (params (Stat :type "/Game/CombatSystem/Blueprints/Enums/E_Stats Enum" :default "NewEnumerator0") (Value :type "Float (double-precision)") (`bShouldRegenerate?` :type Boolean :default true))
  (`self.SetCurrentStatValue` (`local.Stat`) (`KismetMathLibrary.FClamp` (+ (`self.GetCurrentStatValue` (`local.Stat`)) Value) 0.0 (`self.GetMaxStatValue` (`local.Stat`))))
  (if (`local.bShouldRegenerate?`)
    (`self.StartRegen` (`local.Stat`))))

(fn `RegenStamina`
  (`self.SetCurrentStatValue` "NewEnumerator2" (`KismetMathLibrary.FClamp` (+ (`self.GetCurrentStatValue` "NewEnumerator2") (`self.StaminaRegenRate`)) 0.0 (`self.GetMaxStatValue` "NewEnumerator2")))
  (if (>= (`self.GetCurrentStatValue` "NewEnumerator2") (`self.GetMaxStatValue` "NewEnumerator2"))
    (`KismetSystemLibrary.K2_ClearTimer` null "RegenStamina")))

(fn `SetBaseStatValue`
  (params (Key :type "/Game/CombatSystem/Blueprints/Enums/E_Stats Enum" :default "NewEnumerator0") (Value :type "Float (double-precision)"))
  (`BlueprintMapLibrary.Map_Add` (`self.BaseStats`) Key (make `/Game/CombatSystem/Blueprints/Structs/F_BaseStat` Value)))

(fn `SetCurrentStatValue`
  (params (StatType :type "/Game/CombatSystem/Blueprints/Enums/E_Stats Enum" :default "NewEnumerator0") (Value :type "Float (double-precision)"))
  (`BlueprintMapLibrary.Map_Add` (`self.CurrentStats`) StatType Value)
  (`self.OnCurrentStatValueUpdated` (`local.StatType`) (`local.Value`)))

(fn `SetMaxStatValue`
  (params (Key :type "/Game/CombatSystem/Blueprints/Enums/E_Stats Enum" :default "NewEnumerator0") (Value :type "Float (double-precision)"))
  (`BlueprintMapLibrary.Map_Add` (`self.BaseStats`) Key (make `/Game/CombatSystem/Blueprints/Structs/F_BaseStat` 0.0 Value)))

(fn `TakeDamage`
  (params (InDamage :type "Float (double-precision)"))
  (locals (L_Damage :type "Float (double-precision)"))
  (bind _returnvalue (* (`local.InDamage`) (/ (`local.InDamage`) (+ (`local.InDamage`) (`self.GetCurrentStatValue` "NewEnumerator3")))))
  (set `local.L_Damage` (`KismetMathLibrary.FClamp` _returnvalue 0.0 _returnvalue))
  (`self.ModifyCurrentStatValue` "NewEnumerator1" (* (`local.L_Damage`) -1.0)))