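; Actor component in the combat system that holds a character's current state and current action as two separate enums.
; Setters ignore unchanged values, firing a Begin dispatcher with the outgoing value and an End dispatcher with the incoming one, the reverse of what their names suggest.
; Getters, resets and match-any checks serve both enums, and Tick prints both values on screen for debugging.
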(event `self.ReceiveTick`
  (params (DeltaSeconds :type "Float (single-precision)"))
  (`KismetSystemLibrary.PrintString` (`KismetStringLibrary.Concat_StrStr` "Current State: " (`|GetEnumeratorNameAsString` (`self.CurrentState`))) true true (struct :`G` 1.0 :`B` 0.387183 :`A` 1.0) 2.0 "CharacterState")
  (`KismetSystemLibrary.PrintString` (`KismetStringLibrary.Concat_StrStr` "Current Character Action: " (`|GetEnumeratorNameAsString` (`self.CurrentCharacterAction`))) true true (struct :`G` 1.0 :`B` 0.387183 :`A` 1.0) 2.0 "CharacterAction"))

(fn `GetCurrentAction`
  (returns (ReturnValue :type "/Game/CombatSystem/Blueprints/Enums/E_CharacterAction Enum"))
  (return (`self.CurrentCharacterAction`)))

(fn `GetCurrentState`
  (returns (ReturnValue :type "/Game/CombatSystem/Blueprints/Enums/E_CharacterState Enum"))
  (return (`self.CurrentState`)))

(fn `IsCurrentActionEqualToAny?`
  (params (ActionsToCheck :type "Array of /Game/CombatSystem/Blueprints/Enums/E_CharacterAction Enum"))
  (returns (ReturnValue :type Boolean))
  (return (`KismetArrayLibrary.Array_Contains` ActionsToCheck (`self.CurrentCharacterAction`))))

(fn `IsCurrentStateEqualToAny?`
  (params (StatesToCheck :type "Array of /Game/CombatSystem/Blueprints/Enums/E_CharacterState Enum"))
  (returns (ReturnValue :type Boolean))
  (return (`KismetArrayLibrary.Array_Contains` StatesToCheck (`self.CurrentState`))))

(fn `ResetCurrentAction`
  (`self.SetCurrentAction` "NewEnumerator0"))

(fn `ResetState`
  (`self.SetState` "NewEnumerator0"))

(fn `SetCurrentAction`
  (params (NewCharacterAction :type "/Game/CombatSystem/Blueprints/Enums/E_CharacterAction Enum" :default "NewEnumerator0"))
  (if (`|EnumInequality` NewCharacterAction (`self.CurrentCharacterAction`))
    (`self.OnCharacterActionBegin` (`self.CurrentCharacterAction`))
    (bind _output_get (set `self.CurrentCharacterAction` (`local.NewCharacterAction`)))
    (`self.OnCharacterActionEnd` _output_get)))

(fn `SetState`
  (params (NewState :type "/Game/CombatSystem/Blueprints/Enums/E_CharacterState Enum" :default "NewEnumerator0"))
  (if (`|EnumInequality` NewState (`self.CurrentState`))
    (`self.OnStateBegin` (`self.CurrentState`))
    (bind _output_get (set `self.CurrentState` (`local.NewState`)))
    (`self.OnStateEnd` _output_get)))