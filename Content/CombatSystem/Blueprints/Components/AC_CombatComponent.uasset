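; Actor component that manages a character's main weapon and combat state in the combat system.
; Setting a new weapon unequips and destroys the previous one before storing the replacement.
; Toggling combat stores the flag and pushes it to the owning character's mesh anim instance through an update message.
; A reset function clears the saved-attack flag and attack index.
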(fn `GetMainWeapon`
  (returns (ReturnValue :type "/Game/CombatSystem/Blueprints/Actors/Weapon/BP_BaseWeapon Object Reference"))
  (return (`self.MainWeapon`)))

(fn `IsCombatEnabled?`
  (returns (ReturnValue :type Boolean))
  (return (`self.bIsCombatEnabled?`)))

(fn `ResetAttack`
  (set `self.bIsAttackSaved?` false)
  (set `self.AttackIndex` 0))

(fn `SetCombatEnabled`
  (params (`bIsCombatEnabled?` :type Boolean))
  (set `self.bIsCombatEnabled?` `bIsCombatEnabled?`)
  (message `/Game/CombatSystem/Blueprints/Interfaces/BI_AnimInstance.UpdateCombatEnabled` (`SkeletalMeshComponent.GetAnimInstance` (`Character.Mesh` (cast `Character` (`self.GetOwner`) :!pure true))) (`self.bIsCombatEnabled?`)))

(fn `SetMainWeapon`
  (params (NewWeapon :type "/Game/CombatSystem/Blueprints/Actors/Weapon/BP_BaseWeapon Object Reference"))
  (`|ExecutionSequence`
    (:`then_0`
      (bind _mainweapon (`self.MainWeapon`)
        (:`then`
          (`/Game/CombatSystem/Blueprints/Actors/BP_BaseEquippable.OnUnEquipped` _mainweapon)
          (`Actor.K2_DestroyActor` _mainweapon))
        (:`else`)))
    (:`then_1`
      (set `self.MainWeapon` (`local.NewWeapon`)))))